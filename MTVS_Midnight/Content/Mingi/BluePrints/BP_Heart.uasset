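; BP_Heart is an actor that displays player health as three heart components, based on PlayerHP from a QuizWidget reference.
; On BeginPlay only, it destroys Heart3, Heart2 or Heart1 when HP equals 2, 1 or 0 respectively.
; Each exact-match check removes just that one heart, and later HP changes are not tracked.
; The graph never assigns QuizWidget, and a cast to it is left unconnected.
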(event EventBeginPlay
  (bind _quizwidget (Variables|Default|GetQuizWidget))
  (Utilities|FlowControl|Sequence
    (:then_0
      (if (== (Variables|/Script/MTVS_Midnight.QuizWidget|GetPlayerHP _quizwidget) 2)
        (Components|DestroyComponent (Variables|Default|GetHeart3))))
    (:then_1
      (if (== (Variables|/Script/MTVS_Midnight.QuizWidget|GetPlayerHP _quizwidget) 1)
        (Components|DestroyComponent (Variables|Default|GetHeart2))))
    (:then_2
      (if (== (Variables|/Script/MTVS_Midnight.QuizWidget|GetPlayerHP _quizwidget) 0)
        (Components|DestroyComponent (Variables|Default|GetHeart1))))))

(event Collision|EventActorBeginOverlap
  (params (OtherActor :type Actor%20Object%20Reference)))

(event EventTick
  (params (DeltaSeconds :type Float%20%28single-precision%29)))

(fn ConstructionScript)